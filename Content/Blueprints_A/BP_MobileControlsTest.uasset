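; Prototype pawn for testing mobile controls and in-game picture capture, with most of its event logic disconnected.
; On possession by a player controller it adds a prototype widget and the controls input mapping context; a debug Q key takes a UI screenshot.
; SavePicture exports a render target as a timestamp-named PNG and records its metadata in a save game.
; Its only call, alongside camera-rotation and capture experiments, sits in unwired nodes.
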(event Input|EnhancedActionEvents|EnhancedInputActionIA_CaptureFrame
  (params (ActionValue :type Boolean) (ElapsedSeconds :type Float%20%28double-precision%29) (TriggeredSeconds :type Float%20%28double-precision%29) (InputAction :type Input%20Action%20Object%20Reference :default "/Game/Blueprints_A/Inputs/IA_CaptureFrame.IA_CaptureFrame")))

(event Input|EnhancedActionEvents|EnhancedInputActionIA_Move
  (params (ActionValue :type Vector%202D%20Structure) (ElapsedSeconds :type Float%20%28double-precision%29) (TriggeredSeconds :type Float%20%28double-precision%29) (InputAction :type Input%20Action%20Object%20Reference :default "/Game/Blueprints_A/Inputs/IA_Move.IA_Move")))

(event EventBeginPlay)

(event Collision|EventActorBeginOverlap
  (params (OtherActor :type Actor%20Object%20Reference)))

(event EventTick
  (params (DeltaSeconds :type Float%20%28single-precision%29)))

(event EventPossessed
  (params (NewController :type Controller%20Object%20Reference))
  (if (Class|Controller|IsPlayerController NewController)
    (bind _asplayer_controller (Utilities|Casting|CastToPlayerController NewController))
    (bind _returnvalue (UserInterface|CreateWidget "/Game/Blueprints_A/WBP_WidgetPrototypeTest.WBP_WidgetPrototypeTest_C" _asplayer_controller))
    (UserInterface|Viewport|AddtoPlayerScreen _returnvalue)
    (Input|AddMappingContext (PlayerController|LocalPlayerSubsystems|GetEnhancedInputLocalPlayerSubsystem) "/Game/Blueprints_A/Inputs/IMC_Controls.IMC_Controls" 0 "(bIgnoreAllPressedKeysUntilRelease=True,bForceImmediately=False,bNotifyUserSettings=False)")))

(event Input|KeyboardEvents|DebugKeyQ
  (params (Key :type Key%20Structure) (ActionValue :type Input%20Action%20Value%20Structure))
  (:Pressed
    (Development|ExecuteConsoleCommand "Shot showui" 0)))

(event Input|MouseEvents|MiddleMouseButton
  (params (Key :type Key%20Structure)))

(event Input|KeyboardEvents|Acceleration
  (params (AxisValue :type Vector :default "0, 0, 0")))

(fn ConstructionScript)

(fn SavePicture
  (params (picture :type Texture%20Render%20Target%202D%20Object%20Reference) (name :type String) (description :type String) (tags :type Array%20of%20Strings) (isFavorite :type Boolean) (ratio :type ENUM_Ratio%20Enum :default "NewEnumerator0") (zoom :type Float%20%28double-precision%29) (filter :type DS%20Image%20Filter%20Structure))
  (bind _returnvalue (Class|KismetSystemLibrary|GetProjectSavedDirectory))
  (bind _picturessaveslotname (LocalVariables|GetPicturesSaveSlotName))
  (bind _output_get (LocalVariables|SetPictureID (Class|KismetMathLibrary|ToUnixTimestamp (Math|DateTime|UTCNow))))
  (Rendering|ExportRenderTarget picture _returnvalue (Utilities|String|Append (Utilities|String|ToString(Integer) _output_get) ".png"))
  (Utilities|FlowControl|Sequence
    (:then_0
      (bind _returnvalue_2 (SaveGame|DoesSaveGameExist _picturessaveslotname))
      (if _returnvalue_2
        (bind _returnvalue_3 (SaveGame|LoadGamefromSlot _picturessaveslotname))
        (LocalVariables|SetSaveGameObject _returnvalue_3)
        (else
          (bind _returnvalue_4 (SaveGame|CreateSaveGameObject "/Game/Saving/BP_SaveStateTest.BP_SaveStateTest_C"))
          (LocalVariables|SetSaveGameObject _returnvalue_4))))
    (:then_1
      (Default|SavePicture (.AsBP%20Save%20State%20Test (Utilities|Casting|CastToBP_SaveStateTest (LocalVariables|GetSaveGameObject))) (Utilities|Struct|MakeDS_ImageData _output_get (Utilities|String|Append _returnvalue (Utilities|String|Append (Utilities|String|ToString(Integer) _output_get) ".png")) name description tags isFavorite (Utilities|Struct|MakeDS_ImageMetadata ratio zoom (Math|DateTime|UTCNow)) filter) (.AsBP%20Save%20State%20Test (Utilities|Casting|CastToBP_SaveStateTest (LocalVariables|GetSaveGameObject))) (LocalVariables|GetPicturesSaveSlotName)))))