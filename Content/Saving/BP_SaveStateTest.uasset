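; BP_SaveStateTest is a test Blueprint for saving picture data to a named save slot.
; SavePicture loads the slot or creates a BP_SaveStateTest save object, but uses neither result.
; It then appends the picture to its own PictureData and writes the passed-in SaveGameObject to the slot.
; GetPictureData is a stub returning empty defaults for picture metadata and image settings, ignoring the Id.
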(fn SavePicture
  (params (Picture :type DS%20Image%20Data%20Structure%20%28by%20ref%29) (SaveGameObject :type BP%20Save%20State%20Test%20Object%20Reference) (SaveSlotName :type String))
  (LocalVariables|SetPicturesSaveSlotName SaveSlotName)
  (Utilities|FlowControl|Sequence
    (:then_0
      ;[0.15 0.15 0.15 0.5] Load save
      (bind _returnvalue (SaveGame|DoesSaveGameExist (LocalVariables|GetPicturesSaveSlotName)))
      (if _returnvalue
        (SaveGame|LoadGamefromSlot (LocalVariables|GetPicturesSaveSlotName))
        (else
          (SaveGame|CreateSaveGameObject "BP_SaveStateTest_C"))))
    (:then_1
      ;[0.15 0.15 0.15 0.5] Save
      (Utilities|Array|Add (Variables|Default|GetPictureData) Picture)
      (SaveGame|SaveGametoSlot SaveGameObject (LocalVariables|GetPicturesSaveSlotName)))))

(fn GetPictureData
  (params (id :type Integer))
  (return "" "" "" "" false "NewEnumerator0" 0.0 0.0 0.0 0.0))