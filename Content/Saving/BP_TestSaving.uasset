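; Test actor that exercises the BP_SaveStateTest save game and its picture records on BeginPlay.
; It loads the "Test" slot if present, otherwise creates a save, calls SavePicture and writes the slot.
; It then prints the project saved directories, followed by a loop meant to print each picture's timestamp in Montreal time.
; That loop has no array connected, and a second save branch never runs.
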(event EventBeginPlay
  (Utilities|FlowControl|Sequence
    (:then_0
      ;[0.15 0.15 0.15 0.5] Load save
      (bind _returnvalue (SaveGame|DoesSaveGameExist "Test"))
      (Development|PrintString (Utilities|String|ToString(Boolean) _returnvalue) true true "(R=1.000000,G=0.000000,B=0.000145,A=1.000000)" 1e+02)
      (if _returnvalue
        (bind _returnvalue_2 (SaveGame|LoadGamefromSlot "Test"))
        (bind _asbp_save_state_test (Utilities|Casting|CastToBP_SaveStateTest _returnvalue_2))
        (Variables|Default|SetSaveState _asbp_save_state_test)))
    (:then_1
      ;[0.15 0.15 0.15 0.5] Save picture
      (bind _returnvalue_3 (SaveGame|DoesSaveGameExist "Test"))
      (if (not _returnvalue_3)
        ;;[0.15 0.15 0.15 0.5] If save doesn't exist
        (bind _returnvalue_4 (SaveGame|CreateSaveGameObject "/Game/Saving/BP_SaveStateTest.BP_SaveStateTest_C"))
        (bind _output_get (Variables|Default|SetSaveState _returnvalue_4))
        (Default|SavePicture _output_get)
        (SaveGame|SaveGametoSlot _output_get "Test")))
    (:then_2
      ;[0.15 0.15 0.15 0.5] save dir
      (Development|PrintString (Class|KismetSystemLibrary|GetProjectSavedDirectory) true true "(R=1.000000,G=0.000000,B=0.000145,A=1.000000)" 1e+02)
      (Development|PrintString (Class|BlueprintPathsLibrary|ProjectSavedDir) true true "(R=1.000000,G=0.000000,B=0.000145,A=1.000000)" 1e+02))
    (:then_3
      ;[0.15 0.15 0.15 0.5] Print datas
      (for _array_element 0
        (bind _time (Default|GetPictureData (Variables|Default|GetSaveState) _array_element))
        (Development|PrintString (Utilities|String|Append (Utilities|String|ToString(Integer) _array_element) ": " (Utilities|String|ToString(Text) (Class|KismetTextLibrary|AsTimeZoneDateTimeDateTime _time "Montreal" "Short" "Medium"))) true true "(R=0.088070,G=0.000000,B=1.000000,A=1.000000)" 1e+02)))))

(event Collision|EventActorBeginOverlap
  (params (OtherActor :type Actor%20Object%20Reference)))

(event EventTick
  (params (DeltaSeconds :type Float%20%28single-precision%29)))

(fn ConstructionScript)